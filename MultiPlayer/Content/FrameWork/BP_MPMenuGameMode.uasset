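; Game mode for the multiplayer menu that tracks connected players and keeps their lobby views updated.
; New players in the Lobby Menu level are added to the player list, then told to create the lobby menu and run initial setup.
; UpdateLobby rebuilds the profile list and pushes names or the selected level to each BP_MenuController, as flagged.
; Logout removes the player and refreshes names for those remaining.
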(event `self.K2_OnLogout`
  (params (ExitingController :type "Controller Object Reference"))
  (bind _asbp_menu_controller (cast `/Game/FrameWork/BP_MenuController` ExitingController))
  (`KismetArrayLibrary.Array_RemoveItem` (`self.AllConnectedPlayers`) _asbp_menu_controller)
  (`self.UpdateLobby` true))

(event `self.HandleStartingNewPlayer`
  (params (NewPlayer :type "PlayerController Object Reference"))
  (bind _returnvalue (`GameplayStatics.GetCurrentLevelName` true))
  (switch `string` _returnvalue
    (:`Lobby_Menu`
      (bind _asbp_menu_controller (cast `/Game/FrameWork/BP_MenuController` NewPlayer))
      (`KismetArrayLibrary.Array_Add` (`self.AllConnectedPlayers`) _asbp_menu_controller)
      (`/Game/FrameWork/BP_MenuController.CreateLobbyMenu` _asbp_menu_controller)
      (`/Game/FrameWork/BP_MenuController.InitialSetup` _asbp_menu_controller))))

(event `self.ReceiveBeginPlay`)

(event `UpdateLobby`
  (params (PlayerNames :type Boolean) (LevelSelection :type Boolean))
  (`KismetArrayLibrary.Array_Clear` (`self.PlayerProfiles`))
  (for (_array_element _array_index) (`self.AllConnectedPlayers`)
    (`KismetArrayLibrary.Array_Set` (`self.PlayerProfiles`) _array_index (`/Game/FrameWork/BP_MenuController.PlayProfile_info` _array_element) true))
  (for _array_element_2 (`self.AllConnectedPlayers`)
    (if PlayerNames
      (`/Game/FrameWork/BP_MenuController.UpdatePlayerNames` _array_element_2 (`self.PlayerProfiles`)))
    (if LevelSelection
      (`/Game/FrameWork/BP_MenuController.UpdateLevelSelection` _array_element_2 (`self.SelectedLevelName`)))))

(fn `UserConstructionScript`)