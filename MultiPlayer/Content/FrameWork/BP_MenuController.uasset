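; Player controller for the multiplayer menu and lobby, with UI-only input and a visible cursor for the local player.
; InitialSetup loads or creates the saved player profile, then ServerUpdateLobby stores it and asks BP_MPMenuGameMode to update the lobby.
; Events create and reuse the lobby and loading widgets and pass player names and level selection to the lobby widget.
; EndClientSession destroys the session and returns to Main_Menu.
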(event `CreateLoadScreen`
  (`self.UiShowLoadScreen`))

(event `BeginPlay`
  (if (`self.IsLocalController`)
    (set `self.bShowMouseCursor` true)
    (`WidgetBlueprintLibrary.SetInputMode_UIOnlyEx` self null)))

(event `EndClientSession`
  (`DestroySessionCallbackProxy.DestroySession` self
    (:`then`
      (`GameplayStatics.OpenLevel` "Main_Menu"))))

(event `CreateLobbyMenu`
  (`self.UiShowLobbyMenu`))

(event `InitialSetup`
  (`self.LoadSavedProfile`)
  (`self.ServerUpdateLobby` (`self.PlayProfile_info`)))

(event `ServerUpdateLobby`
  (params (PlayerProfile :type "/Game/SavedData/S_PlayerProfile Structure"))
  (set `self.PlayProfile_info` PlayerProfile)
  (bind _asbp_mpmenu_game_mode (cast `/Game/FrameWork/BP_MPMenuGameMode` (`GameplayStatics.GetGameMode`)))
  (`/Game/FrameWork/BP_MPMenuGameMode.UpdateLobby` _asbp_mpmenu_game_mode true true))

(event `UpdatePlayerNames`
  (params (PlayerProfiles :type "Array of /Game/SavedData/S_PlayerProfile Structure"))
  (bind _wg_lobbymenu (`self.WG_LobbyMenu`))
  (`/Engine/EditorBlueprintResources/StandardMacros.IsValid` _wg_lobbymenu
    (:`Is Valid`
      (`/Game/Widgets/WD_LobbyMenu.ClearPlayerNames` _wg_lobbymenu)
      (`/Game/Widgets/WD_LobbyMenu.UpdatePlayerNames` _wg_lobbymenu PlayerProfiles))))

(event `UpdateLevelSelection`
  (params (LevelRowName :type Name))
  (bind _wg_lobbymenu (`self.WG_LobbyMenu`))
  (`/Engine/EditorBlueprintResources/StandardMacros.IsValid` _wg_lobbymenu
    (:`Is Valid`
      (`/Game/Widgets/WD_LobbyMenu.UpdateLevelSelection` _wg_lobbymenu LevelRowName))))

(fn `LoadSavedProfile`
  (locals (LocalSlotName :type String :default "PlayerProfile_slot"))
  (`GameplayStatics.DoesSaveGameExist` (`local.LocalSlotName`))
  (if (not true)
    (bind _returnvalue (`GameplayStatics.CreateSaveGameObject` "/Game/SavedData/SG_PlayerProfile.SG_PlayerProfile_C"))
    (`GameplayStatics.SaveGameToSlot` _returnvalue (`local.LocalSlotName`)))
  (bind _returnvalue_2 (`GameplayStatics.LoadGameFromSlot` (`local.LocalSlotName`)))
  (bind _assg_player_profile (cast `/Game/SavedData/SG_PlayerProfile` _returnvalue_2))
  (set `self.PlayProfile_info` (`/Game/SavedData/SG_PlayerProfile.PlayerProfile` _assg_player_profile))
  (return))

(fn `UiShowLoadScreen`
  (`WidgetLayoutLibrary.RemoveAllWidgets`)
  (`/Engine/EditorBlueprintResources/StandardMacros.IsValid` (`self.WG_LoadScreen`)
    (:`Is Valid`
      _)
    (:`Is Not Valid`
      (bind _returnvalue (`|CreateWidget` "/Game/Widgets/WD_Loading.WD_Loading_C" self))
      (set `self.WG_LoadScreen` _returnvalue)))
  (`UserWidget.AddToViewport` (`self.WG_LoadScreen`) 0)
  (return))

(fn `UiShowLobbyMenu`
  (`/Engine/EditorBlueprintResources/StandardMacros.IsValid` (`self.WG_LobbyMenu`)
    (:`Is Valid`
      _)
    (:`Is Not Valid`
      (bind _returnvalue (`|CreateWidget` "/Game/Widgets/WD_LobbyMenu.WD_LobbyMenu_C" self))
      (set `self.WG_LobbyMenu` _returnvalue)))
  (`UserWidget.AddToViewport` (`self.WG_LobbyMenu`) 0)
  (return))

(fn `UserConstructionScript`)